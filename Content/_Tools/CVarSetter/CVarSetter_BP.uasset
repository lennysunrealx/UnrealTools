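; CVarSetter is a utility Blueprint that applies a configurable set of console commands from its construction script.
; The construction script runs each entry of the CVarSetA array as a console command and prints it.
; When DisableMessages is set, both the construction script and BeginPlay run DisableAllScreenMessages to hide on-screen debug messages.
; BeginPlay does not reapply the CVarSetA commands.
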(event EventBeginPlay
  (if (Variables|Default|GetDisableMessages?)
    ;[1 0.02127 0.008355 0.5] Disable debug messages
    (Development|ExecuteConsoleCommand "DisableAllScreenMessages" 0)))

(event Collision|EventActorBeginOverlap
  (params (OtherActor :type Actor%20Object%20Reference)))

(event EventTick
  (params (DeltaSeconds :type Float%20%28single-precision%29)))

(fn ConstructionScript
  (if (Variables|Default|GetDisableMessages?)
    ;[1 0.02127 0.008355 0.5] Disable debug messages
    (Development|ExecuteConsoleCommand "DisableAllScreenMessages" 0))
  (for _array_element (Variables|Default|GetCVarSetA)
    (Development|ExecuteConsoleCommand _array_element 0)
    (Development|PrintString _array_element)))